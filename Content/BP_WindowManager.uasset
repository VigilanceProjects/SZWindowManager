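; Window manager actor that hosts a toggleable (N key) overlay of UI windows and persists their layout across sessions.
; On start it creates WBP_WindowsMain, then after a delay adds windows from the WindowDA records and restores position, size and state from JSON.
; Losing window focus triggers a delayed save of that JSON.
; UpdateMA hides the overlay and disables player input during online battles or in match rooms.
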(event `self.ReceiveBeginPlay`
  (`self.Initialize`))

(event `Key|N` :consume false :overrideparent false
  (params (Key :type "Key Structure"))
  (:`Pressed`
    (set `self.WantMainWBPVisible` (not (`self.WantMainWBPVisible`)))
    (`Widget.SetVisibility` (`self.WBPWindowsMain`) (select `bool` (`self.WantMainWBPVisible`) :`false` "Collapsed" :`true` "SelfHitTestInvisible" :!type "ESlateVisibility Enum"))))

(event `OnAnyWBPWindowFocusLost`
  (`KismetSystemLibrary.Delay` 5.0)
  (`self.WriteSavedDataJSON`))

(fn `AddWindowsFromRecords`
  (bind _records (`/WindowManager/WindowsDataAsset.Records` (`self.WindowDA`)))
  (bind _keys (`BlueprintMapLibrary.Map_Keys` _records))
  (for _array_element _keys
    (`self.AddWindowToWindowMainWBP` _array_element (`BlueprintMapLibrary.Map_Find` _records _array_element))))

(fn `AddWindowToWindowMainWBP`
  (params (Key :type Name) (Data :type "/WindowManager/S_WindowsDataAsset Structure"))
  (`/WindowManager/WBP_WindowsMain.AddWindow` (`self.WBPWindowsMain`) Key Data))

(fn `InitializeBindings`
  (add `/WindowManager/WBP_WindowsMain.OnAnyWindowFocusLost` (`self.WBPWindowsMain`) (`|CreateDelegate` :!event `OnAnyWBPWindowFocusLost`)))

(fn `InitializeTimers`
  (`KismetSystemLibrary.K2_SetTimerDelegate` (`|CreateDelegate` :!event `UpdateMA`) 1.0 true))

(fn `ReadSavedDataJSON`
  (returns (WindowsSavedData :type "Array of /WindowManager/S_WindowSavedData Structure") (Success :type Boolean))
  (locals (JSONObjects :type "Array of JsonObjectWrapper Structure") (Result :type "Array of /WindowManager/S_WindowSavedData Structure"))
  (bind (_outjsonobject _returnvalue) (`JsonBlueprintFunctionLibrary.FromFile` (make `FilePath` (`self.SavedDataPath`))))
  (if _returnvalue
    (bind _outjsonstring (`JsonBlueprintFunctionLibrary.ToString` _outjsonobject))
    (bind _outjsonobject_2 (`JsonBlueprintFunctionLibrary.FromString` _outjsonstring))
    (bind _outvalue (`|GetJsonField` _outjsonobject_2 "array"))
    (bind _output_get (set `local.JSONObjects` _outvalue))
    (for _array_element _output_get
      (bind _outvalue_2 (`|GetJsonField` _array_element "key"))
      (bind _outvalue_3 (`|GetJsonField` _array_element "position"))
      (bind _outvalue_4 (`|GetJsonField` _array_element "size"))
      (bind _outvalue_5 (`|GetJsonField` _array_element "state"))
      (`KismetArrayLibrary.Array_Add` (`local.Result`) (make `/WindowManager/S_WindowSavedData` _outvalue_2 _outvalue_3 _outvalue_4 _outvalue_5)))
    (return (`local.Result`) true)))

(fn `SetMA`
  (params (Disabled :type Boolean))
  (bind _returnvalue (`GameplayStatics.GetPlayerController` 0))
  (bind _wantmainwbpvisible (`self.WantMainWBPVisible`))
  (bind _wbpwindowsmain (`self.WBPWindowsMain`))
  (if Disabled
    (`self.DisableInput` self _returnvalue)
    (`Widget.SetVisibility` _wbpwindowsmain "Collapsed")
    (else
      (`self.EnableInput` self _returnvalue)
      (if (not (== _wantmainwbpvisible (`Widget.IsVisible` (`self.WBPWindowsMain`))))
        (`Widget.SetVisibility` _wbpwindowsmain (select `bool` _wantmainwbpvisible :`false` "Collapsed" :`true` "SelfHitTestInvisible" :!type "ESlateVisibility Enum"))))))

(fn `UpdateMA`
  (bind _returnvalue (`SSBlueprintFunctionLibrary.GetKoratGameInstance`))
  (`/Engine/EditorBlueprintResources/StandardMacros.IsValid` _returnvalue
    (:`Is Valid`
      (bind _returnvalue_2 (`GameplayStatics.GetActorOfClass` "/Script/SS.SSPlayerMatchRoomController"))
      (bind _output_get (set `self.IsOB` (or (`KismetSystemLibrary.IsValid` _returnvalue_2) (and (`SSGameInstance.GetOnlineBattleFlg` _returnvalue) (`|EnumInequality` (`SSGameInstance.GetBattleOnlineMode` _returnvalue))))))
      (`self.SetMA` _output_get))
    (:`Is Not Valid`
      (set `self.IsOB` false))))

(fn `UpdateWindowsFromSavedData`
  (params (WindowsSavedData :type "Array of /WindowManager/S_WindowSavedData Structure"))
  (locals (Records :type "Map of Name to /WindowManager/S_WindowsDataAsset Structure") (Key :type Name))
  (bind _value (`BlueprintMapLibrary.Map_Find` (`/WindowManager/WBP_WindowsMain.KeysToWindows` (`self.WBPWindowsMain`)) (`local.Key`)))
  (set `local.Records` (`/WindowManager/WindowsDataAsset.Records` (`self.WindowDA`)))
  (for _array_element WindowsSavedData
    (bind (_key _position _size _state) (break `/WindowManager/S_WindowSavedData` _array_element))
    (set `local.Key` _key)
    (if (`.ReturnValue` (`BlueprintMapLibrary.Map_Find` (`local.Records`) (`local.Key`)))
      (`/WindowManager/WBP_Window.SetWindowPosition` _value _position)
      (`/WindowManager/WBP_Window.SetWindowSize` _value _size)
      (`/WindowManager/WBP_Window.SetWindowState` _value _state))))

(fn `UserConstructionScript`
  (`parent.UserConstructionScript`))

(fn `WriteSavedDataJSON`
  (locals (JSONStr :type String :default "{\"array\":["))
  (bind _jsonstr (`local.JSONStr`))
  (bind _values (`BlueprintMapLibrary.Map_Values` (`/WindowManager/WBP_WindowsMain.KeysToWindows` (`self.WBPWindowsMain`))))
  (for (_array_element _array_index) _values
    (bind _returnvalue (`/WindowManager/WBP_Window.GetSelfSlotAsCanvasPanel` _array_element))
    (bind _outjsonstring (`|StructToJsonString` (make `/WindowManager/S_WindowSavedData` (`/WindowManager/WBP_Window.Key` _array_element) (`CanvasPanelSlot.GetPosition` _returnvalue) (`CanvasPanelSlot.GetSize` _returnvalue) (`/WindowManager/WBP_Window.State` _array_element))))
    (set `local.JSONStr` (`KismetMathLibrary.SelectString` (`KismetStringLibrary.Concat_StrStr` _jsonstr _outjsonstring) (`KismetStringLibrary.Concat_StrStr` _jsonstr "," _outjsonstring) (== _array_index 0))))
  (set `local.JSONStr` (`KismetStringLibrary.Concat_StrStr` (`local.JSONStr`) "]}"))
  (bind (_outjsonobject _returnvalue_2) (`JsonBlueprintFunctionLibrary.FromString` (`local.JSONStr`)))
  (if _returnvalue_2
    (`JsonBlueprintFunctionLibrary.ToFile` _outjsonobject (make `FilePath` (`self.SavedDataPath`)))))